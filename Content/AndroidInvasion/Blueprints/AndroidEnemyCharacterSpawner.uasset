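; Destructible spawner that periodically creates enemy androids in the Android Invasion game.
; On BeginPlay a looping timer with a random start delay spawns an AndroidEnemyCharacter at the child actor's location while enabled, with random gender.
; Each impact decrements a hit counter, and at zero the spawner destroys itself with an explosion sound.
; No cap limits how many androids it spawns.
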(event Custom|OnTimerEnds
  ;[1 1 1] Al comienzo del juego, establece una alarma cada SpawnTime segundos. Cuando toca, elige un sexo al azar y crear un androide enemigo de ese tipo
  ; Hay que añadir un control para no generar infinitos robots, cada generador puede controlar lo que ha generado él, o haber un control general...
  (if (Variables|Default|GetEnabled)
    (Game|SpawnActorfromClass "/Game/AndroidInvasion/Blueprints/AndroidEnemyCharacter.AndroidEnemyCharacter_C" (Math|Conversions|ToTransform(Vector) (Transformation|GetWorldLocation (Variables|Default|GetChildActor))) "Undefined" 0 (Math|Random|RandomBool) 0)))

(event EventBeginPlay
  ;[1 1 1] Al comienzo del juego, establece una alarma cada SpawnTime segundos. Cuando toca, elige un sexo al azar y crear un androide enemigo de ese tipo
  ; Hay que añadir un control para no generar infinitos robots, cada generador puede controlar lo que ha generado él, o haber un control general...
  (Utilities|Time|SetTimerbyEvent (delegate Custom|OnTimerEnds) (Variables|Default|GetSpawnTime) true (Math|Random|RandomFloatinRange 1.0 6.0)))

(event EventImpact
  (params (Projectile :type Actor%20Object%20Reference))
  ;[1 1 1] Si me disparan lo suficiente, exploto
  (bind _result (Math|Integer|DecrementInt (Variables|Default|GetHits))
    (:%20%20
      (if (<= _result 0)
        (Actor|DestroyActor)
        (Audio|PlaySoundatLocation "/Game/StarterContent/Audio/Explosion01.Explosion01" (Transformation|GetActorLocation) "0, 0, 0" 1.0 1.0 0.0 0 0 0)))))

(fn ConstructionScript)