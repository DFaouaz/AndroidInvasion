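; AndroidDoor is a door Blueprint that opens while objects are inside its Collision volume and closes once they leave.
; Begin and end overlap events keep a running count of occupants.
; Opening is instant, with no animation: the Door component is hidden and its collision disabled.
; When the count drops to zero or below, the Door becomes visible and solid again.
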(event OnComponentBeginOverlap(Collision)
  (params (OverlappedComponent :type Primitive%20Component%20Object%20Reference) (OtherActor :type Actor%20Object%20Reference) (OtherComp :type Primitive%20Component%20Object%20Reference) (OtherBodyIndex :type Integer) (bFromSweep :type Boolean) (SweepResult :type Hit%20Result%20Structure%20%28by%20ref%29))
  (bind _door (Variables|Default|GetDoor))
  ;[1 1 1] Si algo entra en el radio de acción de la puerta o es golpeada, se abre... y si deja de haber objetos en el radio de acción (o pasa un tiempo tras haber sido golpeada, y tampoco hay objetos) se cierra.
  (Math|Integer|IncrementInt (Variables|Default|GetCount)
    (:%20%20
      (Rendering|SetVisibility _door false false)
      (Collision|SetCollisionEnabled _door "NoCollision"))))

(event OnComponentEndOverlap(Collision)
  (params (OverlappedComponent :type Primitive%20Component%20Object%20Reference) (OtherActor :type Actor%20Object%20Reference) (OtherComp :type Primitive%20Component%20Object%20Reference) (OtherBodyIndex :type Integer))
  (bind _door (Variables|Default|GetDoor))
  ;[1 1 1] Si algo entra en el radio de acción de la puerta o es golpeada, se abre... y si deja de haber objetos en el radio de acción (o pasa un tiempo tras haber sido golpeada, y tampoco hay objetos) se cierra.
  (Math|Integer|DecrementInt (Variables|Default|GetCount)
    (:%20%20
      (if (<= (Variables|Default|GetCount) 0)
        (Rendering|SetVisibility _door true false)
        (Collision|SetCollisionEnabled _door "QueryAndPhysics")))))

(fn ConstructionScript)