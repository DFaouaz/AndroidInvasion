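; AndroidLamp is a lamp actor for the Android Invasion game that shows one of three colors: red, blue or green.
; The construction script applies the material instance matching its Color variable to the static mesh.
; On BeginPlay it picks a random Color and reapplies the matching material, so the color set in the editor is replaced at runtime.
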(event EventBeginPlay
  (bind _staticmeshcomponent (Variables|Debug|GetStaticMeshComponent))
  (Variables|Default|SetColor (.OutItem (Utilities|Array|Random (Utilities|Array|MakeArray "NewEnumerator0" "NewEnumerator1" "NewEnumerator2"))))
  (switch Utilities|FlowControl|Switch|SwitchonAndroidColor (Variables|Default|GetColor)
    (:NewEnumerator0
      (Rendering|Material|SetMaterial _staticmeshcomponent 0 "/Game/AndroidInvasion/Materials/MI_RedAndroidLamp.MI_RedAndroidLamp"))
    (:NewEnumerator1
      (Rendering|Material|SetMaterial _staticmeshcomponent 0 "/Game/AndroidInvasion/Materials/MI_BlueAndroidLamp.MI_BlueAndroidLamp"))
    (:NewEnumerator2
      (Rendering|Material|SetMaterial _staticmeshcomponent 0 "/Game/AndroidInvasion/Materials/MI_GreenAndroidLamp.MI_GreenAndroidLamp"))))

(fn ConstructionScript
  (bind _staticmeshcomponent (Variables|Debug|GetStaticMeshComponent))
  ;[1 1 1] Construir la lámpara con el material correspondiente a su color
  (switch Utilities|FlowControl|Switch|SwitchonAndroidColor (Variables|Default|GetColor)
    (:NewEnumerator0
      (Rendering|Material|SetMaterial _staticmeshcomponent 0 "/Game/AndroidInvasion/Materials/MI_RedAndroidLamp.MI_RedAndroidLamp"))
    (:NewEnumerator1
      (Rendering|Material|SetMaterial _staticmeshcomponent 0 "/Game/AndroidInvasion/Materials/MI_BlueAndroidLamp.MI_BlueAndroidLamp"))
    (:NewEnumerator2
      (Rendering|Material|SetMaterial _staticmeshcomponent 0 "/Game/AndroidInvasion/Materials/MI_GreenAndroidLamp.MI_GreenAndroidLamp"))))