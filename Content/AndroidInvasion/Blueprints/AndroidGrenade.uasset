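; Grenade actor that explodes after a set fuse time or as soon as it hits an actor implementing the Android interface.
; A DoOnce gates the blast, which plays particles and sound, hides the mesh and sets a short lifespan.
; Damage is applied by repeatedly sending ImpactMessage to each Android overlapping the explosion sphere.
; Hits on other physics bodies push them with a scaled impulse.
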(event OnComponentHit(SphereCollision)
  (params (HitComponent :type Primitive%20Component%20Object%20Reference) (OtherActor :type Actor%20Object%20Reference) (OtherComp :type Primitive%20Component%20Object%20Reference) (NormalImpulse :type Vector :default "0, 0, 0") (Hit :type Hit%20Result%20Structure%20%28by%20ref%29))
  ;[1 1 1] Cuando choco contra algo, si es un cuerpo físico, empujarlo... y si no, pues nada, ahí me quedo.
  (if (Utilities|DoesObjectImplementInterface OtherActor "/Game/AndroidInvasion/Blueprints/Android.Android_C")
    ;[1 1 1] REVISAR: Nada más empezar a existir, cuento Duration segundos y exploto, con partículas, sonido e impactando a todos los androides con los que esté solapado
    (Utilities|FlowControl|DoOnce false
      (:Completed
        (Components|Activation|Activate (Variables|Default|GetExplosionPS) false)
        (Audio|PlaySoundatLocation "/Game/StarterContent/Audio/Explosion02.Explosion02" (Transformation|GetActorLocation) "0, 0, 0" 1.0 1.0 0.0 0 0 0)
        (for _array_element (Collision|GetOverlappingActors (Variables|Default|GetSphereExplosion) 0 :!class /Script/Engine.PrimitiveComponent)
          (if (Utilities|DoesObjectImplementInterface _array_element "/Game/AndroidInvasion/Blueprints/Android.Android_C")
            (for _index (range 0 (Variables|Default|GetDamage))
              (Class|Android|Impact(Message) _array_element self))))
        (Actor|SetLifeSpan 2.5)
        (Rendering|SetVisibility (Variables|Default|GetSphere) false false)))
    (elif (Utilities|Enum|Equal(Enum) (Collision|GetCollisionObjectType OtherComp) "ECC_PhysicsBody")
      (Physics|AddImpulse OtherComp (* NormalImpulse (Variables|Default|GetImpulse)) "None" true))))

(event EventBeginPlay
  ;[1 1 1] REVISAR: Nada más empezar a existir, cuento Duration segundos y exploto, con partículas, sonido e impactando a todos los androides con los que esté solapado
  (Utilities|FlowControl|Delay (Variables|Default|GetDuration))
  (Utilities|FlowControl|DoOnce false
    (:Completed
      (Components|Activation|Activate (Variables|Default|GetExplosionPS) false)
      (Audio|PlaySoundatLocation "/Game/StarterContent/Audio/Explosion02.Explosion02" (Transformation|GetActorLocation) "0, 0, 0" 1.0 1.0 0.0 0 0 0)
      (for _array_element (Collision|GetOverlappingActors (Variables|Default|GetSphereExplosion) 0 :!class /Script/Engine.PrimitiveComponent)
        (if (Utilities|DoesObjectImplementInterface _array_element "/Game/AndroidInvasion/Blueprints/Android.Android_C")
          (for _index (range 0 (Variables|Default|GetDamage))
            (Class|Android|Impact(Message) _array_element self))))
      (Actor|SetLifeSpan 2.5)
      (Rendering|SetVisibility (Variables|Default|GetSphere) false false))))

(fn ConstructionScript)