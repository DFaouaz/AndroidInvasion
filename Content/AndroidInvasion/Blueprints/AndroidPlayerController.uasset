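; Player controller for AndroidInvasion that caches the possessed AndroidPlayerCharacter and forwards movement, look, jump and fire input to it.
; It tracks the selected projectile, toggling between normal shots and grenades, and G refills both ammo counts.
; Left Shift sprints by scaling walk speed, with Tick draining stamina, dropping speed at empty and regenerating when not sprinting.
; Game won and lost events show the cursor and notify AndroidHUD.
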(event Custom|OnGameWon
  ;[1 1 1] Cuando me avisen de que he ganado, muestro el ratón (me faltaría hacer foco en los botones) y saco el menú de victoria
  (Variables|Default|SetbShowMouseCursor true)
  (Default|OnGameWon (CallFunction|GetAndroidHUD)))

(event Custom|OnGameLost
  ;[1 1 1] Cuando me avisen de que he muerto, muestro el ratón (me faltaría hacer foco en los botones) y saco el menú de partida perdida
  (Variables|Default|SetbShowMouseCursor true)
  (Default|OnGameLost (CallFunction|GetAndroidHUD)))

(event EventPossess
  (params (PossessedPawn :type Pawn%20Object%20Reference))
  ;[1 1 1] Android Player Controller - Cuando posea algo, asumo que es el AndroidCharacter y me lo guardo (en realidad esto lo podría obviar)
  (bind _asandroid_player_character (Utilities|Casting|CastToAndroidPlayerCharacter PossessedPawn))
  (Variables|Default|SetAndroidCharacter _asandroid_player_character))

(event EventTick
  (params (DeltaSeconds :type Float%20%28single-precision%29))
  ;[1 1 1] Añadir la posibilidad de correr y gastar energia (recuperarla por no correr)
  (if (Variables|Default|GetSprinting)
    (if (> (Variables|/Game/AndroidInvasion/Blueprints/AndroidPlayerCharacter.AndroidPlayerCharacter_C|GetStamina (Variables|Default|GetAndroidCharacter)) 0.0)
      (Variables|/Game/AndroidInvasion/Blueprints/AndroidPlayerCharacter.AndroidPlayerCharacter_C|SetStamina (Variables|Default|GetAndroidCharacter) (- (Variables|/Game/AndroidInvasion/Blueprints/AndroidPlayerCharacter.AndroidPlayerCharacter_C|GetStamina (Variables|Default|GetAndroidCharacter)) (* (Variables|Default|GetStaminaLoss) DeltaSeconds)))
      (else
        (Variables|/Script/Engine.CharacterMovementComponent|SetMaxWalkSpeed (Variables|/Script/Engine.Character|GetCharacterMovement (Variables|Default|GetAndroidCharacter)) (Variables|Default|GetInitialMaxSpeed))))
    (elif (< (Variables|/Game/AndroidInvasion/Blueprints/AndroidPlayerCharacter.AndroidPlayerCharacter_C|GetStamina (Variables|Default|GetAndroidCharacter)) 1.0)
      (Variables|/Game/AndroidInvasion/Blueprints/AndroidPlayerCharacter.AndroidPlayerCharacter_C|SetStamina (Variables|Default|GetAndroidCharacter) (+ (* (Variables|Default|GetStaminaGain) DeltaSeconds) (Variables|/Game/AndroidInvasion/Blueprints/AndroidPlayerCharacter.AndroidPlayerCharacter_C|GetStamina (Variables|Default|GetAndroidCharacter)))))))

(event EventBeginPlay
  (Variables|Default|SetInitialMaxSpeed (Class|MovementComponent|GetMaxSpeed (Variables|/Script/Engine.Character|GetCharacterMovement (Variables|Default|GetAndroidCharacter))))
  (Variables|Default|SetCurrentProjectile "/Game/AndroidInvasion/Blueprints/AndroidProjectile.AndroidProjectile_C"))

(event Input|ActionEvents|InputActionJump
  (params (Key :type Key%20Structure :default "None"))
  (bind _androidcharacter (Variables|Default|GetAndroidCharacter))
  ;[1 1 1] Salto
  (:Pressed
    (Character|Jump _androidcharacter))
  (:Released
    (Character|StopJumping _androidcharacter)))

(event Input|ActionEvents|InputActionFire
  (params (Key :type Key%20Structure :default "None"))
  ;[1 1 1] Si pulsan disparar, le digo al cuerpo que dispare
  (:Pressed
    (Default|Fire (Variables|Default|GetAndroidCharacter) (Variables|Default|GetCurrentProjectile))))

(event Input|ActionEvents|InputActionSwapProjectile
  (params (Key :type Key%20Structure :default "None"))
  ;[1 1 1] Cambiar de proyectiles entre granadas y munición normal (llevar la cuenta aparte
  (:Pressed
    (if (== (Variables|Default|GetCurrentProjectile) "/Game/AndroidInvasion/Blueprints/AndroidProjectile.AndroidProjectile_C")
      (Variables|Default|SetCurrentProjectile "/Game/AndroidInvasion/Blueprints/AndroidGrenade.AndroidGrenade_C")
      (else
        (Variables|Default|SetCurrentProjectile "/Game/AndroidInvasion/Blueprints/AndroidProjectile.AndroidProjectile_C")))))

(event Input|AxisEvents|InputAxisMoveForward
  (params (AxisValue :type Float%20%28single-precision%29))
  (bind _androidcharacter (Variables|Default|GetAndroidCharacter))
  ;[1 1 1] Movimiento con el stick (o teclado)
  (Pawn|Input|AddMovementInput _androidcharacter (Transformation|GetActorForwardVector _androidcharacter) AxisValue false))

(event Input|AxisEvents|InputAxisMoveRight
  (params (AxisValue :type Float%20%28single-precision%29))
  (bind _androidcharacter (Variables|Default|GetAndroidCharacter))
  ;[1 1 1] Movimiento con el stick (o teclado)
  (Pawn|Input|AddMovementInput _androidcharacter (Transformation|GetActorRightVector _androidcharacter) AxisValue false))

(event Input|AxisEvents|InputAxisTurn
  (params (AxisValue :type Float%20%28single-precision%29))
  ;[1 1 1] Rotaciones con el ratón
  (Pawn|Input|AddControllerYawInput (Variables|Default|GetAndroidCharacter) AxisValue))

(event Input|AxisEvents|InputAxisLookUp
  (params (AxisValue :type Float%20%28single-precision%29))
  ;[1 1 1] Rotaciones con el ratón
  (Pawn|Input|AddControllerPitchInput (Variables|Default|GetAndroidCharacter) AxisValue))

(event Input|AxisEvents|InputAxisLookUpRate
  (params (AxisValue :type Float%20%28single-precision%29))
  (bind _androidcharacter (Variables|Default|GetAndroidCharacter))
  ;[1 1 1] Rotaciones con el stick (o teclado)
  (Pawn|Input|AddControllerPitchInput _androidcharacter (* (Utilities|Time|GetWorldDeltaSeconds) AxisValue (Variables|/Game/AndroidInvasion/Blueprints/AndroidPlayerCharacter.AndroidPlayerCharacter_C|GetBaseLookUpRate _androidcharacter))))

(event Input|AxisEvents|InputAxisTurnRate
  (params (AxisValue :type Float%20%28single-precision%29))
  (bind _androidcharacter (Variables|Default|GetAndroidCharacter))
  ;[1 1 1] Rotaciones con el stick (o teclado)
  (Pawn|Input|AddControllerYawInput _androidcharacter (* (Variables|/Game/AndroidInvasion/Blueprints/AndroidPlayerCharacter.AndroidPlayerCharacter_C|GetBaseTurnRate _androidcharacter) AxisValue (Utilities|Time|GetWorldDeltaSeconds))))

(event Input|KeyboardEvents|G
  (params (Key :type Key%20Structure :default "None"))
  (bind _androidcharacter (Variables|Default|GetAndroidCharacter))
  ;[1 1 1] Recargar maximo de balas en la municion
  (:Pressed
    (Variables|/Game/AndroidInvasion/Blueprints/AndroidPlayerCharacter.AndroidPlayerCharacter_C|SetAmmo _androidcharacter (Variables|/Game/AndroidInvasion/Blueprints/AndroidPlayerCharacter.AndroidPlayerCharacter_C|GetMaxAmmo _androidcharacter))
    (Variables|/Game/AndroidInvasion/Blueprints/AndroidPlayerCharacter.AndroidPlayerCharacter_C|SetGrenades _androidcharacter (Variables|/Game/AndroidInvasion/Blueprints/AndroidPlayerCharacter.AndroidPlayerCharacter_C|GetMaxGrenades _androidcharacter))))

(event Input|KeyboardEvents|LeftShift
  (params (Key :type Key%20Structure :default "None"))
  (bind _androidcharacter (Variables|Default|GetAndroidCharacter))
  (bind _charactermovement (Variables|/Script/Engine.Character|GetCharacterMovement _androidcharacter))
  ;[1 1 1] Añadir la posibilidad de correr y gastar energia (recuperarla por no correr)
  (:Pressed
    (Variables|Default|SetSprinting true)
    (if (> (Variables|/Game/AndroidInvasion/Blueprints/AndroidPlayerCharacter.AndroidPlayerCharacter_C|GetStamina (Variables|Default|GetAndroidCharacter)) 0.0)
      (Variables|/Script/Engine.CharacterMovementComponent|SetMaxWalkSpeed _charactermovement (* (Variables|Default|GetInitialMaxSpeed) (Variables|Default|GetSprintModifierRatio)))
      (else
        (Variables|Default|SetSprinting false :!label _label)
        (Variables|/Script/Engine.CharacterMovementComponent|SetMaxWalkSpeed _charactermovement (Variables|Default|GetInitialMaxSpeed)))))
  (:Released
    (goto _label)))

(fn ConstructionScript)

(fn GetAndroidHUD
  ;[1 1 1] Devuelve el HUD, asumiendo que siempre es un Android HUD
  (return (.AsAndroid%20HUD (Utilities|Casting|CastToAndroidHUD (HUD|GetHUD)))))