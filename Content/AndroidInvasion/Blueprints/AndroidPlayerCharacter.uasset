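; First-person player character for Android Invasion that tracks health, ammo and grenades, filling both ammo counts on BeginPlay.
; Damage lowers Health and notifies AndroidGameMode of death at zero or below.
; One Fire event serves both projectile types, checking the matching count before playing the montage and sound, spawning the projectile along the camera rotation and decrementing that count.
; The construction script attaches the gun to the arms' GripPoint socket.
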(event Custom|Fire
  (params (ProjectileClass :type Actor%20Class%20Reference))
  (bind _returnvalue (== ProjectileClass "/Game/AndroidInvasion/Blueprints/AndroidProjectile.AndroidProjectile_C"))
  (bind _sphere (Variables|Default|GetSphere))
  (bind _firstpersoncamera (Variables|MyCharacter|GetFirstPersonCamera))
  (bind _returnvalue_2 (Transformation|GetWorldRotation _firstpersoncamera))
  (bind _returnvalue_3 (Transformation|GetWorldLocation _sphere))
  ;[1 1 1] Disparar proyectil (de munición normal, podría hacerse lo mismo sean granadas o proyectiles... o bien usar raycast para munición
  (if _returnvalue
    (if (> (Variables|Default|GetAmmo) 0)
      (Animation|Montage|MontagePlay (Components|SkeletalMesh|GetAnimInstance (Variables|MyCharacter|GetMesh2P)) "/Game/FirstPerson/Animations/FirstPersonFire_Montage.FirstPersonFire_Montage" 1.0 "MontageLength" 0.0 true :!label _label)
      (Game|SpawnActorfromClass ProjectileClass (Math|Transform|MakeTransform (+ _returnvalue_3 (Math|Vector|RotateVector (Variables|Default|GetGunOffset) _returnvalue_2)) _returnvalue_2) "Undefined" 0 (Class|PawnMovementComponent|GetPawnOwner (Variables|Character|GetCharacterMovement)))
      (Audio|PlaySoundatLocation "/Game/FirstPerson/Audio/FirstPersonTemplateWeaponFire02.FirstPersonTemplateWeaponFire02" _returnvalue_3 "0, 0, 0" 1.0 1.0 0.0 0 0 0)
      (if _returnvalue
        (Math|Integer|DecrementInt (Variables|Default|GetAmmo))
        (else
          (Math|Integer|DecrementInt (Variables|Default|GetGrenades))))
      (else
        (Development|PrintString "NO AMMO" :!label _label_2)))
    (elif (> (Variables|Default|GetGrenades) 0)
      (goto _label)
      (else
        (goto _label_2)))))

(event Game|Damage|EventAnyDamage
  (params (Damage :type Float%20%28single-precision%29) (DamageType :type Damage%20Type%20Object%20Reference) (InstigatedBy :type Controller%20Object%20Reference) (DamageCauser :type Actor%20Object%20Reference))
  ;[1 1 1] Si recibo daño, lo descuento de mi salud... y si llega a ser cero o menos, aviso al GM que me muero
  (bind _output_get (Variables|Default|SetHealth (- (Variables|Default|GetHealth) Damage)))
  (if (<= _output_get 0.0)
    (bind _asandroid_game_mode (Utilities|Casting|CastToAndroidGameMode (Game|GetGameMode)))
    (Default|OnPlayerDead _asandroid_game_mode)))

(event EventBeginPlay
  (Variables|Default|SetAmmo (Variables|Default|GetMaxAmmo))
  (Variables|Default|SetGrenades (Variables|Default|GetMaxGrenades)))

(fn ConstructionScript
  ;[1 1 1] Se adjunta el arma en el GripPoint
  (Transformation|AttachComponentToComponent (Variables|Default|GetFP_Gun) (Variables|MyCharacter|GetMesh2P) "GripPoint" "SnapToTarget" "SnapToTarget" "SnapToTarget" true))