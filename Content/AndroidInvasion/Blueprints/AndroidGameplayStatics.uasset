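; AndroidGameplayStatics is a Blueprint function library that gives typed access to the core framework objects of the Android Invasion game.
; Each function fetches the standard player controller, game instance, player character or game mode and casts it to its Android-specific class.
; The casts assume the types always match, and the player lookups always use player index 0.
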(fn GetAndroidPlayerController
  ;[1 1 1] Devuelve el controlador, asumiendo que siempre es un Android Player Controller
  (return (.AsAndroid%20Player%20Controller (Utilities|Casting|CastToAndroidPlayerController (Game|GetPlayerController 0)))))

(fn GetAndroidGameInstance
  ;[1 1 1] Devuelve la instancia, asumiendo que siempre es un Android Game Instance
  (return (.AsAndroid%20Game%20Instance (Utilities|Casting|CastToAndroidGameInstance (Game|GetGameInstance)))))

(fn GetAndroidPlayerCharacter
  ;[1 1 1] Devuelve el personaje del jugador, asumiendo que siempre es un Android Player Character
  (return (.AsAndroid%20Player%20Character (Utilities|Casting|CastToAndroidPlayerCharacter (Game|GetPlayerCharacter 0)))))

(fn GetAndroidGameMode
  ;[1 1 1] Devuelve el modo, asumiendo que siempre es un Android Game Mode
  (return (.AsAndroid%20Game%20Mode (Utilities|Casting|CastToAndroidGameMode (Game|GetGameMode)))))