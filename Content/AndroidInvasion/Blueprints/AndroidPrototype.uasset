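; AndroidPrototype is an Android Invasion actor representing a destructible android prototype with a skeletal mesh, fire and spark effects.
; On its first Impact event, it switches the mesh to physics simulation, activates the fire, deactivates both spark effects and notifies the Android Game Mode of its destruction.
; The mesh's physics-simulation state doubles as the guard against repeated destruction.
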(event EventImpact
  (params (Projectile :type Actor%20Object%20Reference))
  (bind _skeletalmeshcomponent (Variables|Default|GetSkeletalMeshComponent))
  ;[1 1 1] Si recibo un impacto (y aún no estoy simulando física), empiezo a simular físicas en mi esqueleto, activo el fuego y aviso al Game Mode
  (if (not (Physics|IsSimulatingPhysics _skeletalmeshcomponent "None"))
    (Physics|SetSimulatePhysics _skeletalmeshcomponent true)
    (Components|Activation|Activate (Variables|Default|GetFire) false)
    (Components|Activation|Deactivate (Variables|Default|GetSparks1))
    (Components|Activation|Deactivate (Variables|Default|GetSparks2))
    (Default|OnPrototypeDestroyed (CallFunction|GetAndroidGameMode))))

(fn ConstructionScript)