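; BP_AmmoPackage is a pickup that refills either normal ammo or grenades for the player, chosen by the IsNormalAmmo flag.
; The construction script uses that flag to set the amount and tint the cube green for ammo or red for grenades.
; When an AndroidPlayerCharacter overlaps the cube, it adds the amount to the matching count, clamped to that character's maximum, then destroys itself.
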(event OnComponentBeginOverlap(Cube)
  (params (OverlappedComponent :type Primitive%20Component%20Object%20Reference) (OtherActor :type Actor%20Object%20Reference) (OtherComp :type Primitive%20Component%20Object%20Reference) (OtherBodyIndex :type Integer) (bFromSweep :type Boolean) (SweepResult :type Hit%20Result%20Structure%20%28by%20ref%29))
  (bind _asandroid_player_character (Utilities|Casting|CastToAndroidPlayerCharacter OtherActor))
  (if (Variables|Default|GetIsNormalAmmo)
    (Variables|/Game/AndroidInvasion/Blueprints/AndroidPlayerCharacter.AndroidPlayerCharacter_C|SetAmmo _asandroid_player_character (Math|Integer|Clamp(Integer) (+ (Variables|/Game/AndroidInvasion/Blueprints/AndroidPlayerCharacter.AndroidPlayerCharacter_C|GetAmmo _asandroid_player_character) (Variables|Default|GetAmmoCount)) 0 (Variables|/Game/AndroidInvasion/Blueprints/AndroidPlayerCharacter.AndroidPlayerCharacter_C|GetMaxAmmo _asandroid_player_character)))
    (else
      (Variables|/Game/AndroidInvasion/Blueprints/AndroidPlayerCharacter.AndroidPlayerCharacter_C|SetGrenades _asandroid_player_character (Math|Integer|Clamp(Integer) (+ (Variables|/Game/AndroidInvasion/Blueprints/AndroidPlayerCharacter.AndroidPlayerCharacter_C|GetGrenades _asandroid_player_character) (Variables|Default|GetAmmoCount)) 0 (Variables|/Game/AndroidInvasion/Blueprints/AndroidPlayerCharacter.AndroidPlayerCharacter_C|GetMaxGrenades _asandroid_player_character)))))
  (Actor|DestroyActor))

(event EventBeginPlay)

(event EventTick
  (params (DeltaSeconds :type Float%20%28single-precision%29)))

(fn ConstructionScript
  (bind _cube (Variables|Default|GetCube))
  (if (Variables|Default|GetIsNormalAmmo)
    (Variables|Default|SetAmmoCount 10)
    (Rendering|Material|SetMaterial _cube 0 "/Game/AndroidInvasion/Materials/MI_GreenAndroidLamp.MI_GreenAndroidLamp")
    (else
      (Variables|Default|SetAmmoCount 2)
      (Rendering|Material|SetMaterial _cube 0 "/Game/AndroidInvasion/Materials/MI_RedAndroidLamp.MI_RedAndroidLamp"))))