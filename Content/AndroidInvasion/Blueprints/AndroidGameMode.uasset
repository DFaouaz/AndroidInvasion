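; Game mode for Android Invasion that tracks prototype targets, scales difficulty and handles winning and losing.
; On BeginPlay it counts AndroidPrototype actors, divides each enemy spawner's SpawnTime by the game instance's level, and calls a cinematic trigger inside that loop.
; Destroying the last prototype plays a sound, notifies the player controller of victory and removes "ExitFloor"-tagged actors.
; Player death pauses the game, resets the level counter and notifies the controller of defeat.
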(event Custom|OnPlayerDead
  ;[1 1 1] Cuando matan al jugador, pauso, reinicio el nivel por el que vamos (¡permadeth, otra vez al nivel inicial!) y le digo al controlador que ha perdido.
  (Game|SetGamePaused true)
  (Game|GetCurrentLevelName true)
  (Variables|/Game/AndroidInvasion/Blueprints/AndroidGameInstance.AndroidGameInstance_C|SetLevel (CallFunction|GetAndroidGameInstance) 0)
  (bind _asandroid_player_controller (Utilities|Casting|CastToAndroidPlayerController (Game|GetPlayerController 0)))
  (Default|OnGameLost _asandroid_player_controller))

(event Custom|OnPrototypeDestroyed
  ;[1 1 1] Cuando se destruye un prototipo, se reduce 1 de la cantidad de los que quedan... y si llega a 0, le digo al controlador que ha ganado, y además también hago un cambio en el mapa: busco el primer actor etiquetado como "ExitFloor" y lo elimino, para dejar acceso libre a la salida
  (bind _result (Math|Integer|DecrementInt (Variables|Default|GetTargetsLeft))
    (:%20%20
      (if (<= _result 0)
        (Audio|PlaySound2D "/Game/StarterContent/Audio/Starter_Background_Cue.Starter_Background_Cue" 1.0 1.0 0.0 0 0)
        (Default|OnGameWon (CallFunction|GetAndroidPlayerController))
        (bind _outactors (Actor|GetAllActorswithTag "ExitFloor"))
        (bind _array_element (Utilities|Array|ForEachLoopwithBreak _outactors)
          (:LoopBody
            (Actor|DestroyActor _array_element)))))))

(event EventBeginPlay
  ;[1 1 1] Android Game Mode - Nada más empezar un nivel, contabilizo todos los prototipos androides que hay, y guardo el valor total.
  ; Además se ajusta la dificultad según el número de nivel (por ahora únicamente se divide el tiempo de los generadores entre el número del nivel (manteniendo un lapso mínimo de 1 segundo entre generación y generación)
  (bind _outactors (Actor|GetAllActorsOfClass "/Game/AndroidInvasion/Blueprints/AndroidPrototype.AndroidPrototype_C"))
  (bind _output_get (Variables|Default|SetTotalTargets (Utilities|Array|Length _outactors)))
  (Variables|Default|SetTargetsLeft _output_get)
  (bind _outactors_2 (Actor|GetAllActorsOfClass "/Game/AndroidInvasion/Blueprints/AndroidEnemyCharacterSpawner.AndroidEnemyCharacterSpawner_C"))
  (for _array_element _outactors_2
    (Variables|/Game/AndroidInvasion/Blueprints/AndroidEnemyCharacterSpawner.AndroidEnemyCharacterSpawner_C|SetSpawnTime _array_element (/ (Variables|/Game/AndroidInvasion/Blueprints/AndroidEnemyCharacterSpawner.AndroidEnemyCharacterSpawner_C|GetSpawnTime _array_element) (Math|Conversions|ToFloat(Integer) (Variables|/Game/AndroidInvasion/Blueprints/AndroidGameInstance.AndroidGameInstance_C|GetLevel (CallFunction|GetAndroidGameInstance)))))
    (Default|CallTriggerCinametic)))

(fn ConstructionScript)