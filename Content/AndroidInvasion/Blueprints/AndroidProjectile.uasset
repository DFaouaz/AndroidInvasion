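; AndroidProjectile is a projectile actor that reacts to whatever it hits, then destroys itself.
; Targets implementing the Android interface receive an ImpactMessage with the projectile as argument, leaving the response to them.
; Otherwise, a valid PhysicsBody component gets an impulse from the projectile's velocity at its location.
; The construction script randomly gives the Ray component a red, blue or green lamp material.
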(event Collision|EventHit
  (params (MyComp :type Primitive%20Component%20Object%20Reference) (Other :type Actor%20Object%20Reference) (OtherComp :type Primitive%20Component%20Object%20Reference) (bSelfMoved :type Boolean) (HitLocation :type Vector :default "0, 0, 0") (HitNormal :type Vector :default "0, 0, 0") (NormalImpulse :type Vector :default "0, 0, 0") (Hit :type Hit%20Result%20Structure%20%28by%20ref%29))
  ;[1 1 1] Cuando choco contra algo, si es un Prototipo, IMPACTARLO... si no, si es un cuerpo físico, empujarlo... y si no, pues nada
  (Utilities|FlowControl|Sequence
    (:then_0
      (if (Utilities|DoesObjectImplementInterface Other "/Game/AndroidInvasion/Blueprints/Android.Android_C")
        (Class|Android|Impact(Message) Other self)
        (else
          ;;[1 1 1] Tengo que ver si el componente es VÁLIDO
          (Utilities|IsValid OtherComp
            (:Is%20Valid
              (if (Utilities|Enum|Equal(Enum) (Collision|GetCollisionObjectType OtherComp) "ECC_PhysicsBody")
                (Physics|AddImpulseatLocation OtherComp (Transformation|GetVelocity) (Transformation|GetActorLocation) "None")))))))
    (:then_1
      (Actor|DestroyActor))))

(fn ConstructionScript
  (bind _ray (Variables|Default|GetRay))
  (switch Utilities|FlowControl|Switch|SwitchonAndroidColor (.OutItem (Utilities|Array|Random (Utilities|Array|MakeArray "NewEnumerator0" "NewEnumerator1" "NewEnumerator2")))
    (:NewEnumerator0
      (Rendering|Material|SetMaterial _ray 0 "/Game/AndroidInvasion/Materials/MI_RedAndroidLamp.MI_RedAndroidLamp"))
    (:NewEnumerator1
      (Rendering|Material|SetMaterial _ray 0 "/Game/AndroidInvasion/Materials/MI_BlueAndroidLamp.MI_BlueAndroidLamp"))
    (:NewEnumerator2
      (Rendering|Material|SetMaterial _ray 0 "/Game/AndroidInvasion/Materials/MI_GreenAndroidLamp.MI_GreenAndroidLamp"))))