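; HUD for the AndroidInvasion game, managing the intro sequence, crosshair, header, level notice and end-game menus.
; BeginPlay disables input and gravity, plays a cinematic below level 2, then shows UMG widgets and restores control after a brief level notice.
; DrawHUD draws the crosshair at screen center unless the intro or win menu is active.
; Win and loss events add their menus, with game over first removing any win menu.
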(event Custom|OnGameWon
  ;[1 1 1] Cuando me lo pidan, muestro el menú de victoria (no impide el juego y se queda ahí, persistente)
  (bind _returnvalue (UserInterface|CreateWidget "/Game/AndroidInvasion/UI/WinMenu.WinMenu_C"))
  (UserInterface|Viewport|AddtoViewport _returnvalue 0)
  (Variables|Default|SetWinMenu true))

(event Custom|HideWinMenu
  ;[1 1 1] Intentar quitar el menú de victoria si está puesto
  (if (Variables|Default|GetWinMenu)
    (bind _foundwidgets (Widget|GetAllWidgetsOfClass "/Game/AndroidInvasion/UI/WinMenu.WinMenu_C" true))
    (Widget|RemovefromParent (Utilities|Array|Get(acopy) _foundwidgets))
    (Variables|Default|SetWinMenu false)))

(event Custom|OnGameLost
  ;[1 1 1] Cuando me lo pidan, muestro el menú de partida perdida (intento quitar el de victoria si está puesto, para que no estén ambos)
  (CallFunction|HideWinMenu)
  (bind _returnvalue (UserInterface|CreateWidget "/Game/AndroidInvasion/UI/GameOverMenu.GameOverMenu_C"))
  (UserInterface|Viewport|AddtoViewport _returnvalue 0))

(event Custom|CinameticFinished
  (bind _asandroid_player_controller (CallFunction|GetAndroidPlayerController))
  ;[1 1 1] Al comenzar el jueg, si el nivel es inferior al 2, toca cinemática: se inhabilita la entrada, se pone gravedad a cero (para dejar al personaje en el aire) y se hace la cinemática.
  ; Luego, ya se pone el HUD normal, la parte hecha con UMG... y al ratito un mensaje informando del nivel en el que estás (debería transicionar poco a poco, pero bueno)
  (bind _returnvalue (UserInterface|CreateWidget "/Game/AndroidInvasion/UI/HUDHeader.HUDHeader_C"))
  (UserInterface|Viewport|AddtoViewport _returnvalue 0)
  (bind _returnvalue_2 (UserInterface|CreateWidget "/Game/AndroidInvasion/UI/LevelInfo.LevelInfo_C"))
  (UserInterface|Viewport|AddtoViewport _returnvalue_2 0)
  (Utilities|FlowControl|Delay 2.0)
  (Widget|RemovefromParent _returnvalue_2)
  (Input|EnableInput _asandroid_player_controller 0)
  (Variables|/Script/Engine.CharacterMovementComponent|SetGravityScale (Variables|/Script/Engine.Character|GetCharacterMovement (Variables|/Game/AndroidInvasion/Blueprints/AndroidPlayerController.AndroidPlayerController_C|GetAndroidCharacter _asandroid_player_controller)) 1.0)
  (Variables|Default|SetCinematics false))

(event EventBeginPlay
  (bind _asandroid_game_instance (CallFunction|GetAndroidGameInstance))
  (bind _asandroid_player_controller (CallFunction|GetAndroidPlayerController))
  (bind _asandroid_game_mode (CallFunction|GetAndroidGameMode))
  (bind _asandroid_player_controller_2 (CallFunction|GetAndroidPlayerController))
  ;[1 1 1] Al comenzar el jueg, si el nivel es inferior al 2, toca cinemática: se inhabilita la entrada, se pone gravedad a cero (para dejar al personaje en el aire) y se hace la cinemática.
  ; Luego, ya se pone el HUD normal, la parte hecha con UMG... y al ratito un mensaje informando del nivel en el que estás (debería transicionar poco a poco, pero bueno)
  (Utilities|IsValid _asandroid_game_instance
    (:Is%20Valid
      (if (< (Variables|/Game/AndroidInvasion/Blueprints/AndroidGameInstance.AndroidGameInstance_C|GetLevel _asandroid_game_instance) 2)
        (Utilities|FlowControl|Sequence
          (:then_0
            (Input|DisableInput _asandroid_player_controller_2 0 :!label _label)
            (Variables|/Script/Engine.CharacterMovementComponent|SetGravityScale (Variables|/Script/Engine.Character|GetCharacterMovement (Variables|/Game/AndroidInvasion/Blueprints/AndroidPlayerController.AndroidPlayerController_C|GetAndroidCharacter _asandroid_player_controller_2)) 0.0))
          (:then_1
            (Default|CallTriggerCinametic _asandroid_game_mode)
            (EventDispatchers|BindEventtoCinematicFinished _asandroid_game_mode (delegate Custom|CinameticFinished))
            (Variables|Default|SetCinematics true :!label _label_2)))
        (else
          (Utilities|FlowControl|Sequence
            (:then_0
              (goto _label))
            (:then_1
              (goto _label_2))
            (:then_2
              (bind _returnvalue (UserInterface|CreateWidget "/Game/AndroidInvasion/UI/HUDHeader.HUDHeader_C"))
              (UserInterface|Viewport|AddtoViewport _returnvalue 0)
              (bind _returnvalue_2 (UserInterface|CreateWidget "/Game/AndroidInvasion/UI/LevelInfo.LevelInfo_C"))
              (UserInterface|Viewport|AddtoViewport _returnvalue_2 0)
              (Utilities|FlowControl|Delay 2.0)
              (Widget|RemovefromParent _returnvalue_2)
              (Input|EnableInput _asandroid_player_controller 0)
              (Variables|/Script/Engine.CharacterMovementComponent|SetGravityScale (Variables|/Script/Engine.Character|GetCharacterMovement (Variables|/Game/AndroidInvasion/Blueprints/AndroidPlayerController.AndroidPlayerController_C|GetAndroidCharacter _asandroid_player_controller)) 1.0)
              (Variables|Default|SetCinematics false))))))))

(event EventDrawHUD
  (params (SizeX :type Integer) (SizeY :type Integer))
  ;[1 1 1] Dibujo mediante Slate una mirilla en el centro de la escena (siempre que no esté mostrando cinemáticas)
  (if (and (not (Variables|Default|GetCinematics)) (not (Variables|Default|GetWinMenu)))
    (Class|HUD|DrawTextureSimple "/Game/FirstPerson/Textures/FirstPersonCrosshair.FirstPersonCrosshair" (Math|Conversions|ToFloat(Integer) (/ SizeX 2)) (Math|Conversions|ToFloat(Integer) (/ SizeY 2)) 1.0 false)))

(fn ConstructionScript)